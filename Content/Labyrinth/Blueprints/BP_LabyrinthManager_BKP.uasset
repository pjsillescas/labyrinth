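; Labyrinth manager that outlines a recursive procedural layout of randomly sized rooms linked by corridors on a tile grid.
; GenerateLabyrinth branches once or twice per room, choosing a non-reversing direction and recursing until Count runs out.
; CheckRoom tests tile occupancy with vertical line traces but is never called here.
; CreateRoom only returns false, halting generation immediately, while CreateCorridor and CheckCorridor are unfinished stubs.
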(event EventBeginPlay)

(event Collision|EventActorBeginOverlap
  (params (OtherActor :type Actor%20Object%20Reference)))

(event EventTick
  (params (DeltaSeconds :type Float%20%28single-precision%29)))

(fn ConstructionScript)

(fn GenerateLabyrinth
  (params (Origin :type Vector%202D%20Structure) (Width :type Float%20%28single-precision%29) (Height :type Float%20%28single-precision%29) (Direction :type E_Direction2%20Enum :default "NewEnumerator0") (Count :type Integer))
  (LocalVariables|SetLOrigin Origin)
  (LocalVariables|SetLWidth Width)
  (LocalVariables|SetLHeight Height)
  (LocalVariables|SetLDir Direction)
  (LocalVariables|SetLCount Count)
  (bind _success (CallFunction|CreateRoom (LocalVariables|GetLOrigin) (LocalVariables|GetLWidth) (LocalVariables|GetLHeight) (LocalVariables|GetLDir)))
  (if (and _success (> (LocalVariables|GetLCount) 0))
    (for _index (range 1 (Math|Random|RandomIntegerinRange 1 2))
      (LocalVariables|SetLLength (Math|Random|RandomIntegerinRange 3 5))
      (bind _newdirection (CallFunction|GetNewDirection (LocalVariables|GetLDir) (LocalVariables|GetLOrigin) (Math|Conversions|ToFloat(Integer) (LocalVariables|GetLLength)) (LocalVariables|GetLWidth) (LocalVariables|GetLHeight)))
      (LocalVariables|SetLDir _newdirection)
      (CallFunction|CreateCorridor (LocalVariables|GetLOrigin) (Math|Conversions|ToFloat(Integer) (LocalVariables|GetLLength)) (LocalVariables|GetLDir) (LocalVariables|GetLWidth) (LocalVariables|GetLHeight))
      (bind _output_get (LocalVariables|SetLPosssibleSizeValues (Utilities|Array|MakeArray 6 8 10)))
      (LocalVariables|SetLNewWidth (CallFunction|GetRandomElementfromArray _output_get))
      (LocalVariables|SetLNewHeight (CallFunction|GetRandomElementfromArray _output_get))
      (Utilities|FlowControl|Sequence
        (:then_0
          (LocalVariables|SetLDeltaX (+ (Math|Conversions|ToFloat(Integer) (LocalVariables|GetLLength)) (Math|Conversions|ToFloat(Integer) (/ (LocalVariables|GetLNewWidth) 2)) (/ (LocalVariables|GetLWidth) 2.0) -1.0)))
        (:then_1
          (LocalVariables|SetLDeltaY (+ (Math|Conversions|ToFloat(Integer) (LocalVariables|GetLLength)) (Math|Conversions|ToFloat(Integer) (/ (LocalVariables|GetLNewHeight) 2)) (/ (LocalVariables|GetLHeight) 2.0) -1.0)))
        (:then_2
          (switch Utilities|FlowControl|Switch|SwitchonE_Direction2 (LocalVariables|GetLDir)
            (:NewEnumerator0
              (LocalVariables|SetLNewOrigin (Math|Vector2D|MakeVector2D (LocalVariables|GetLDeltaX) 0.0)))
            (:NewEnumerator1
              (LocalVariables|SetLNewOrigin (Math|Vector2D|MakeVector2D (* (LocalVariables|GetLDeltaX) -1.0) 0.0)))
            (:NewEnumerator2
              (LocalVariables|SetLNewOrigin (Math|Vector2D|MakeVector2D 0.0 (* (LocalVariables|GetLDeltaY) -1.0))))
            (:NewEnumerator3
              (LocalVariables|SetLNewOrigin (Math|Vector2D|MakeVector2D 0.0 (LocalVariables|GetLDeltaY))))))
        (:then_3
          (LocalVariables|SetLNewOrigin (+ (LocalVariables|GetLNewOrigin) (LocalVariables|GetLOrigin)))
          (CallFunction|GenerateLabyrinth (LocalVariables|GetLNewOrigin) (Math|Conversions|ToFloat(Integer) (LocalVariables|GetLNewWidth)) (Math|Conversions|ToFloat(Integer) (LocalVariables|GetLNewHeight)) (LocalVariables|GetLDir) (- (LocalVariables|GetLCount) 1))))))
  (return))

(fn CreateRoom
  (params (Origin :type Vector%202D%20Structure) (Width :type Float%20%28single-precision%29) (Height :type Float%20%28single-precision%29) (Direction :type E_Direction2%20Enum :default "NewEnumerator0"))
  (return false))

(fn GetNewDirection
  (params (Direction :type E_Direction2%20Enum :default "NewEnumerator0") (Origin :type Vector%202D%20Structure) (Length :type Float%20%28single-precision%29) (Width :type Float%20%28single-precision%29) (Height :type Float%20%28single-precision%29))
  (LocalVariables|SetLDirection Direction)
  (LocalVariables|SetLOrigin Origin)
  (LocalVariables|SetLLength Length)
  (LocalVariables|SetLWidth Width)
  (LocalVariables|SetLHeight Height)
  (bind _output_get (LocalVariables|SetPossibleDirections (Utilities|Array|MakeArray "NewEnumerator0" "NewEnumerator1" "NewEnumerator2" "NewEnumerator3")))
  (Utilities|Array|Shuffle _output_get)
  (bind _array_element (Utilities|Array|ForEachLoopwithBreak _output_get :!label _label)
    (:LoopBody
      (bind _success (CallFunction|CheckCorridor (LocalVariables|GetLOrigin) (LocalVariables|GetLLength) (LocalVariables|GetLDirection) (LocalVariables|GetLWidth) (LocalVariables|GetLHeight)))
      (if (and (Utilities|Enum|NotEqual(Enum) _array_element (CallFunction|GetAntiDirection (LocalVariables|GetLDirection))) _success)
        (LocalVariables|SetLNewDirection _array_element)
        (goto _label Break)))
    (:Completed
      (return (LocalVariables|GetLNewDirection)))))

(fn GetAntiDirection
  (params (Direction :type E_Direction2%20Enum :default "NewEnumerator0"))
  (switch Utilities|FlowControl|Switch|SwitchonE_Direction2 Direction
    (:NewEnumerator0
      (LocalVariables|SetLAntiDirection "NewEnumerator1"))
    (:NewEnumerator1
      (LocalVariables|SetLAntiDirection "NewEnumerator0"))
    (:NewEnumerator2
      (LocalVariables|SetLAntiDirection "NewEnumerator3"))
    (:NewEnumerator3
      (LocalVariables|SetLAntiDirection "NewEnumerator2")))
  (return (LocalVariables|GetLAntiDirection)))

(fn CheckCorridor
  (params (Origin :type Vector%202D%20Structure) (Length :type Float%20%28single-precision%29) (Direction :type E_Direction2%20Enum :default "NewEnumerator0") (Width :type Float%20%28single-precision%29) (Height :type Float%20%28single-precision%29))
  (LocalVariables|SetLLength (+ Length 5.0))
  (Utilities|FlowControl|Sequence
    (:then_0
      (switch Utilities|FlowControl|Switch|SwitchonE_Direction2 Direction))
    (:then_1
      (return (LocalVariables|GetLSuccess)))))

(fn CreateCorridor
  (params (Origin :type Vector%202D%20Structure) (Length :type Float%20%28single-precision%29) (Direction :type E_Direction2%20Enum :default "NewEnumerator0") (Width :type Float%20%28single-precision%29) (Height :type Float%20%28single-precision%29)))

(fn GetRandomElementfromArray
  (params (Array :type Array%20of%20Integers))
  (return (Utilities|Array|Get(acopy) Array (Math|Random|RandomIntegerinRange 0 (- (Utilities|Array|Length Array) 1)))))

(fn CheckRoom
  (params (Origin :type Vector%202D%20Structure) (Width :type Float%20%28single-precision%29) (Height :type Float%20%28single-precision%29) (Direction :type E_Direction2%20Enum :default "NewEnumerator0"))
  (bind _returnvalue (/ Height 2.0))
  (bind _returnvalue_2 (/ Width 2.0))
  (bind _tilesize (Variables|Default|GetTileSize))
  (bind _returnvalue_3 (Math|Conversions|ToFloat(Integer) _tilesize))
  (LocalVariables|SetLOrigin Origin)
  (bind _index (Utilities|FlowControl|ForLoopwithBreak (* (Math|Float|Floor _returnvalue_2) -1) (- (Math|Float|Ceil _returnvalue_2) 1) :!label _label)
    (:LoopBody
      (LocalVariables|SetLi _index)
      (if (LocalVariables|GetLocalSuccess)
        (bind _index_2 (Utilities|FlowControl|ForLoopwithBreak (* (Math|Float|Floor _returnvalue) -1) (- (Math|Float|Ceil _returnvalue) 1) :!label _label_2)
          (:LoopBody
            (LocalVariables|SetLj _index_2)
            (bind _output_get (LocalVariables|SetLTilePosition (Math|Vector2D|MakeVector2D (* (+ (.x (LocalVariables|GetLOrigin)) (Math|Conversions|ToFloat(Integer) (LocalVariables|GetLi))) _returnvalue_3) (* (+ (.y (LocalVariables|GetLOrigin)) (Math|Conversions|ToFloat(Integer) (LocalVariables|GetLj))) _returnvalue_3))))
            (bind _isemptyposition (CallFunction|IsTileEmpty _output_get))
            (if (not _isemptyposition)
              (LocalVariables|SetLocalSuccess false)
              (goto _label_2 Break))))
        (else
          (goto _label Break))))
    (:Completed
      (return (LocalVariables|GetLocalSuccess)))))

(fn IsTileEmpty
  (params (TilePosition :type Vector%202D%20Structure))
  (bind (_x _y) (Math|Vector2D|BreakVector2D TilePosition))
  (bind _returnvalue (Collision|LineTraceByChannel (Math|Vector|MakeVector _x _y (- (Variables|Default|GetZFloor) (LocalVariables|GetLOffset))) (Math|Vector|MakeVector _x _y (+ (Variables|Default|GetZFloor) (LocalVariables|GetLOffset))) "TraceTypeQuery1" false 0 "None"))
  (return (not _returnvalue)))